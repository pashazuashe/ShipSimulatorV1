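; Floatable pawn with a mouse-orbited, scroll-zoomed spring arm camera and keyboard-adjusted Speed and Angle values.
; W/S step Speed and A/D step a limited Angle, both shown as text but not driving movement.
; Tick eases actor yaw toward the velocity direction and applies a zero forward force to the mesh.
; Forward/right axis events are empty, the Speed-scaled force helper is uncalled, and camera-switch nodes are disconnected.
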(event EventBeginPlay
  (Transformation|SetActorRotation (Math|Rotator|MakeRotator 0.0 0.0 0.0)))

(event EventTick
  (params (DeltaSeconds :type Float%20%28single-precision%29))
  (bind _returnvalue (Transformation|GetActorRotation))
  (bind _springarm (Variables|Default|GetSpringArm))
  (bind (_roll _pitch) (Math|Rotator|BreakRotator _returnvalue))
  (Rendering|Components|TextRender|SetText (Variables|Default|GetTextSpeed) (Utilities|Text|ToText(Float) (Variables|Default|GetSpeed) "HalfToEven"))
  (Rendering|Components|TextRender|SetText (Variables|Default|GetTextAngle) (Utilities|Text|ToText(Float) (Variables|Default|GetAngle) "HalfToEven"))
  (Transformation|SetActorRotation (Math|Rotator|MakeRotator _roll _pitch (.yaw (Math|Rotator|Lerp(Rotator) _returnvalue (Math|Conversions|RotationFromXVector (Transformation|GetVelocity)) 0.1 true))))
  (Physics|AddForce (Variables|Default|GetStaticMesh) (* "" (Transformation|GetActorForwardVector)) "None" true)
  (Variables|/Script/Engine.SpringArmComponent|SetTargetArmLength _springarm (- (Variables|/Script/Engine.SpringArmComponent|GetTargetArmLength _springarm) (* (Variables|Default|GetScrollSensivity) (Class|Actor|GetInputAxisKeyValue)))))

(event Input|ActionEvents|InputActionChangeCamera
  (params (Key :type Key%20Structure)))

(event Input|AxisEvents|InputAxisMoveForward
  (params (AxisValue :type Float%20%28single-precision%29)))

(event Input|AxisEvents|InputAxisMoveRight
  (params (AxisValue :type Float%20%28single-precision%29)))

(event Input|AxisEvents|InputAxisMoveMouseX
  (params (AxisValue :type Float%20%28single-precision%29))
  (if (!= AxisValue 0.0)
    (Transformation|AddRelativeRotation (Variables|Default|GetSpringArm) (Math|Rotator|MakeRotator 0.0 0.0 (* AxisValue (Variables|Default|GetSensivity))) false false)))

(event Input|AxisEvents|InputAxisMoveMouseY
  (params (AxisValue :type Float%20%28single-precision%29))
  (if (!= AxisValue 0.0)
    (Transformation|AddRelativeRotation (Variables|Default|GetSpringArm) (Math|Rotator|MakeRotator 0.0 (* AxisValue (Variables|Default|GetSensivity)) 0.0) false false)))

(event Input|KeyboardEvents|W
  (params (Key :type Key%20Structure))
  (:Pressed
    (Variables|Default|SetSpeed (+ 1.0 (Variables|Default|GetSpeed)))))

(event Input|KeyboardEvents|S
  (params (Key :type Key%20Structure))
  (:Pressed
    (Variables|Default|SetSpeed (+ -1.0 (Variables|Default|GetSpeed)))))

(event Input|KeyboardEvents|A
  (params (Key :type Key%20Structure))
  (:Pressed
    (if (> (Variables|Default|GetAngle) -6.0)
      (Variables|Default|SetAngle (+ -1.0 (Variables|Default|GetAngle))))))

(event Input|KeyboardEvents|D
  (params (Key :type Key%20Structure))
  (:Pressed
    (if (< (Variables|Default|GetAngle) 6.0)
      (Variables|Default|SetAngle (+ 1.0 (Variables|Default|GetAngle))))))

(fn ConstructionScript)