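; Debug pawn driven by physics forces on its mesh, with mouse-rotated spring arm and eight toggleable container components.
; Move axes apply acceleration along actor axes; without forward input, Tick pushes backward only when velocity is zero.
; Containers start hidden; E shows and F hides the one at the current index, which increments or decrements on key release.
; The velocity-facing yaw lerp in ChangeRotation is disconnected, and forward force is printed for debugging.
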(event EventBeginPlay
  (Development|SetHiddeninGame (Variables|Default|Getc1) true false)
  (Development|SetHiddeninGame (Variables|Default|Getc2) true false)
  (Development|SetHiddeninGame (Variables|Default|Getc3) true false)
  (Development|SetHiddeninGame (Variables|Default|Getc4) true false)
  (Development|SetHiddeninGame (Variables|Default|Getc5) true false)
  (Development|SetHiddeninGame (Variables|Default|Getc6) true false)
  (Development|SetHiddeninGame (Variables|Default|Getc7) true false)
  (Development|SetHiddeninGame (Variables|Default|Getc8) true false))

(event EventTick
  (params (DeltaSeconds :type Float%20%28single-precision%29))
  (if (not (Variables|Default|GetForwardInput))
    (bind _returnvalue (Physics|GetPhysicsLinearVelocity (Variables|Default|GetStaticMesh) "None"))
    (if (not (Utilities|Operators|NotEqual(!=) :A _returnvalue))
      (Physics|AddForce (Variables|Default|GetStaticMesh) (* (* (Math|Float|Sign(Float) -1.0) (Variables|Default|GetSpeed)) (Transformation|GetActorForwardVector)) "None" true))))

(event Input|AxisEvents|InputAxisMoveForward
  (params (AxisValue :type Float%20%28single-precision%29))
  (bind _returnvalue (Transformation|GetActorForwardVector))
  (bind _speed (Variables|Default|GetSpeed))
  (bind _returnvalue_2 (* AxisValue _speed))
  (bind _returnvalue_3 (* _returnvalue_2 _returnvalue))
  (Physics|AddForce (Variables|Default|GetStaticMesh) _returnvalue_3 "None" true)
  (if (Utilities|Operators|NotEqual(!=) :A _returnvalue_3)
    (Variables|Default|SetForwardInput true)
    (else
      (Variables|Default|SetForwardInput false)))
  (Development|PrintString (Utilities|String|ToString(Vector) _returnvalue_3)))

(event Input|AxisEvents|InputAxisMoveRight
  (params (AxisValue :type Float%20%28single-precision%29))
  (Physics|AddForce (Variables|Default|GetStaticMesh) (* (* AxisValue (Variables|Default|GetAngularSpeed)) (Transformation|GetActorRightVector)) "None" true))

(event Input|AxisEvents|InputAxisMoveMouseX
  (params (AxisValue :type Float%20%28single-precision%29))
  (if (!= AxisValue 0.0)
    (Transformation|AddRelativeRotation (Variables|Default|GetSpringArm) (Math|Rotator|MakeRotator 0.0 0.0 (* AxisValue (Variables|Default|GetSensivity))) false false)))

(event Input|AxisEvents|InputAxisMoveMouseY
  (params (AxisValue :type Float%20%28single-precision%29))
  (if (!= AxisValue 0.0)
    (Transformation|AddRelativeRotation (Variables|Default|GetSpringArm) (Math|Rotator|MakeRotator 0.0 (* AxisValue (Variables|Default|GetSensivity)) 0.0) false false)))

(event Input|KeyboardEvents|E
  (params (Key :type Key%20Structure))
  (:Pressed
    (switch int (Variables|Default|GetContainers)
      (:0
        (Development|SetHiddeninGame (Variables|Default|Getc1) false false))
      (:1
        (Development|SetHiddeninGame (Variables|Default|Getc2) false false))
      (:2
        (Development|SetHiddeninGame (Variables|Default|Getc3) false false))
      (:3
        (Development|SetHiddeninGame (Variables|Default|Getc4) false false))
      (:4
        (Development|SetHiddeninGame (Variables|Default|Getc5) false false))
      (:5
        (Development|SetHiddeninGame (Variables|Default|Getc6) false false))
      (:6
        (Development|SetHiddeninGame (Variables|Default|Getc7) false false))
      (:7
        (Development|SetHiddeninGame (Variables|Default|Getc8) false false))))
  (:Released
    (Variables|Default|SetContainers (+ (Variables|Default|GetContainers) 1))))

(event Input|KeyboardEvents|F
  (params (Key :type Key%20Structure))
  (:Pressed
    (switch int (Variables|Default|GetContainers)
      (:0
        (Development|SetHiddeninGame (Variables|Default|Getc1) true false))
      (:1
        (Development|SetHiddeninGame (Variables|Default|Getc2) true false))
      (:2
        (Development|SetHiddeninGame (Variables|Default|Getc3) true false))
      (:3
        (Development|SetHiddeninGame (Variables|Default|Getc4) true false))
      (:4
        (Development|SetHiddeninGame (Variables|Default|Getc5) true false))
      (:5
        (Development|SetHiddeninGame (Variables|Default|Getc6) true false))
      (:6
        (Development|SetHiddeninGame (Variables|Default|Getc7) true false))
      (:7
        (Development|SetHiddeninGame (Variables|Default|Getc8) true false))))
  (:Released
    (Variables|Default|SetContainers (- (Variables|Default|GetContainers) 1))))

(fn ConstructionScript)

(fn ChangeRotation
  (bind _returnvalue (Transformation|GetActorRotation))
  (bind (_roll _pitch) (Math|Rotator|BreakRotator _returnvalue))
  (Transformation|SetActorRotation (Math|Rotator|MakeRotator _roll _pitch (.yaw (Math|Rotator|Lerp(Rotator) _returnvalue (Math|Conversions|RotationFromXVector (Transformation|GetVelocity)) 0.1 true)))))