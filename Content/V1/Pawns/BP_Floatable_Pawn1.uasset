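; Player-controlled pawn, named as floatable, that moves by physics forces on its static mesh.
; Forward and right axis inputs apply mass-independent forces along the actor's vectors, scaled by separate linear and angular speed variables.
; Tick eases only the yaw toward the velocity direction, so sideways force steers the pawn.
; ChangeCamera flip-flops the camera between two relative locations, and BeginPlay resets the actor rotation.
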(event EventBeginPlay
  (Transformation|SetActorRotation (Math|Rotator|MakeRotator 0.0 0.0 0.0)))

(event EventTick
  (params (DeltaSeconds :type Float%20%28single-precision%29))
  (bind _returnvalue (Transformation|GetActorRotation))
  (bind (_roll _pitch) (Math|Rotator|BreakRotator _returnvalue))
  (Transformation|SetActorRotation (Math|Rotator|MakeRotator _roll _pitch (.yaw (Math|Rotator|Lerp(Rotator) _returnvalue (Math|Conversions|RotationFromXVector (Transformation|GetVelocity)) 0.1 true)))))

(event Input|ActionEvents|InputActionChangeCamera
  (params (Key :type Key%20Structure))
  (bind _camera (Variables|Default|GetCamera))
  (:Pressed
    (Utilities|FlowControl|FlipFlop
      (:A
        (Transformation|SetRelativeLocationAndRotation _camera (Variables|Default|GetCmaera0Loc) "-20.000000,0.000000,0.000000" false false))
      (:B
        (Transformation|SetRelativeLocationAndRotation _camera (Variables|Default|GetCamera1Loc) "0, 0, 0" false false)))))

(event Input|AxisEvents|InputAxisMoveForward
  (params (AxisValue :type Float%20%28single-precision%29))
  (Physics|AddForce (Variables|Default|GetStaticMesh) (* (* AxisValue (Variables|Default|GetSpeed)) (Transformation|GetActorForwardVector)) "None" true))

(event Input|AxisEvents|InputAxisMoveRight
  (params (AxisValue :type Float%20%28single-precision%29))
  (Physics|AddForce (Variables|Default|GetStaticMesh) (* (* AxisValue (Variables|Default|GetAngularSpeed)) (Transformation|GetActorRightVector)) "None" true))

(fn ConstructionScript)