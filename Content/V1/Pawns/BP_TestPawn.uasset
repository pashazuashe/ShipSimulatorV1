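; Test vehicle pawn driven by stepped gear and steering inputs, which loads and uploads four containers at base actors.
; W/S and A/D set target speed and angle; Tick eases current values toward them, yaws the Cube, moves along its forward vector and updates debug text.
; Mouse controls orbit and zoom the spring-arm camera.
; E animates containers from an overlapping BP_LoadBase into their slots; F calls BP_UploadBase, then swaps their materials in sequence.
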(event EventBeginPlay
  ;[0.1373 0.1373 0.1373] Setup material
  (Rendering|SetVisibility (Variables|Default|GetC1) false false)
  (Rendering|SetVisibility (Variables|Default|GetC2) false false)
  (Rendering|SetVisibility (Variables|Default|GetC3) false false)
  (Rendering|SetVisibility (Variables|Default|GetC4) false false))

(event EventTick
  (params (DeltaSeconds :type Float%20%28single-precision%29))
  (bind _angle (Variables|Default|GetAngle))
  (bind _cube (Variables|Default|GetCube))
  (bind _speed (Variables|Default|GetSpeed))
  (bind _speed_2 (Variables|Default|GetSpeed))
  (bind _angle_2 (Variables|Default|GetAngle))
  (bind _relativerotation (Variables|/Script/Engine.SceneComponent|GetRelativeRotation _cube))
  ;[0 0 0] Comment
  (CallFunction|UpdateText)
  ;;[0.1373 0.1373 0.1373] Add Rotation
  (if (> (Variables|Default|GetCurrentSpeed) 0.0)
    (Transformation|SetRelativeRotation _cube (Math|Rotator|MakeRotator 0.0 0.0 (+ (.yaw _relativerotation) (* (Variables|Default|GetCurrentAngle) 0.05))) false false)
    (elif (< (Variables|Default|GetCurrentSpeed) 0.0)
      (Transformation|SetRelativeRotation _cube (Math|Rotator|MakeRotator 0.0 0.0 (+ (.yaw _relativerotation) (* (Variables|Default|GetCurrentAngle) -0.05))) false false)))
  ;;[0.1373 0.1373 0.1373] Add Movement
  (Pawn|Input|AddMovementInput (Math|Vector|GetForwardVector (Variables|Default|GetCube)) (/ (Variables|Default|GetCurrentSpeed) (Variables|Default|GetGearsCount)) false)
  ;;[0.1373 0.1373 0.1373] Change Speed
  (if (> (Variables|Default|GetSpeed) (Variables|Default|GetCurrentSpeed))
    (if (<= (+ (Variables|Default|GetCurrentSpeed) (Variables|Default|GetSpeedAcceleration)) _speed_2)
      (Variables|Default|SetCurrentSpeed (+ (Variables|Default|GetCurrentSpeed) (Variables|Default|GetSpeedAcceleration)))
      (else
        (Variables|Default|SetCurrentSpeed _speed_2)))
    (elif (>= (- (Variables|Default|GetCurrentSpeed) (Variables|Default|GetSpeedAcceleration)) _speed)
      (Variables|Default|SetCurrentSpeed (- (Variables|Default|GetCurrentSpeed) (Variables|Default|GetSpeedAcceleration)))
      (else
        (Variables|Default|SetCurrentSpeed _speed))))
  ;;[0.1373 0.1373 0.1373] Change Angle
  (if (> (Variables|Default|GetAngle) (Variables|Default|GetCurrentAngle))
    (if (<= (+ (Variables|Default|GetCurrentAngle) (Variables|Default|GetAngleAcceleration)) _angle_2)
      (Variables|Default|SetCurrentAngle (+ (Variables|Default|GetCurrentAngle) (Variables|Default|GetAngleAcceleration)))
      (else
        (Variables|Default|SetCurrentAngle _angle_2)))
    (elif (>= (- (Variables|Default|GetCurrentAngle) (Variables|Default|GetAngleAcceleration)) _angle)
      (Variables|Default|SetCurrentAngle (- (Variables|Default|GetCurrentAngle) (Variables|Default|GetAngleAcceleration)))
      (else
        (Variables|Default|SetCurrentAngle _angle)))))

(event Input|AxisEvents|InputAxisMoveMouseX
  (params (AxisValue :type Float%20%28single-precision%29))
  ;[0 0 0] Mouse
  ;;[0.1373 0.1373 0.1373] Mouse X-axis
  (if (!= AxisValue 0.0)
    (Transformation|AddRelativeRotation (Variables|Default|GetSpringArm) (Math|Rotator|MakeRotator 0.0 0.0 (* AxisValue (Variables|Default|GetSensivity))) false false)))

(event Input|AxisEvents|InputAxisMoveMouseY
  (params (AxisValue :type Float%20%28single-precision%29))
  ;[0 0 0] Mouse
  ;;[0.1373 0.1373 0.1373] Mouse Y-axis
  (if (!= AxisValue 0.0)
    (Transformation|AddRelativeRotation (Variables|Default|GetSpringArm) (Math|Rotator|MakeRotator 0.0 (* AxisValue (Variables|Default|GetSensivity)) 0.0) false false)))

(event Input|MouseEvents|MouseWheelAxis
  (params (AxisValue :type Float%20%28single-precision%29))
  (bind _springarm (Variables|Default|GetSpringArm))
  ;[0 0 0] Mouse
  ;;[0.1373 0.1373 0.1373] Scroll wheel
  (if (> (- (Variables|/Script/Engine.SpringArmComponent|GetTargetArmLength _springarm) (* (Variables|Default|GetScrollSensivity) AxisValue)) 6e+02)
    (Variables|/Script/Engine.SpringArmComponent|SetTargetArmLength _springarm (- (Variables|/Script/Engine.SpringArmComponent|GetTargetArmLength _springarm) (* (Variables|Default|GetScrollSensivity) AxisValue)))))

(event Input|KeyboardEvents|W
  (params (Key :type Key%20Structure :default "None"))
  ;[0 0 0] Set Speed & Angle
  ;;[0.1373 0.1373 0.1373] Set Speed
  (:Pressed
    (if (< (Variables|Default|GetSpeed) (Variables|Default|GetGearsCount))
      (Variables|Default|SetSpeed (+ 1.0 (Variables|Default|GetSpeed))))))

(event Input|KeyboardEvents|S
  (params (Key :type Key%20Structure :default "None"))
  ;[0 0 0] Set Speed & Angle
  ;;[0.1373 0.1373 0.1373] Set Speed
  (:Pressed
    (if (not (> (Variables|Default|GetSpeed) (Variables|Default|GetGearsCount)))
      (Variables|Default|SetSpeed (+ -1.0 (Variables|Default|GetSpeed))))))

(event Input|KeyboardEvents|A
  (params (Key :type Key%20Structure :default "None"))
  ;[0 0 0] Set Speed & Angle
  ;;[0.1373 0.1373 0.1373] Set Angle
  (:Pressed
    (if (> (Variables|Default|GetAngle) (* (Variables|Default|GetAnglesCount) -1))
      (Variables|Default|SetAngle (+ -1.0 (Variables|Default|GetAngle))))))

(event Input|KeyboardEvents|D
  (params (Key :type Key%20Structure :default "None"))
  ;[0 0 0] Set Speed & Angle
  ;;[0.1373 0.1373 0.1373] Set Angle
  (:Pressed
    (if (< (Variables|Default|GetAngle) (Variables|Default|GetAnglesCount))
      (Variables|Default|SetAngle (+ 1.0 (Variables|Default|GetAngle))))))

(event Input|KeyboardEvents|E
  (params (Key :type Key%20Structure :default "None"))
  (bind _c1 (Variables|Default|GetC1))
  (bind _c3 (Variables|Default|GetC3))
  (bind _c2 (Variables|Default|GetC2))
  (bind _c4 (Variables|Default|GetC4))
  (bind _tempboxloc (Variables|Default|GetTempBoxLoc))
  ;[0 0 0] Comment
  ;;[0.1373 0.1373 0.1373] Load containers
  (:Pressed
    (for _array_element (Collision|GetOverlappingActors (Variables|Default|GetCapsule) "/Game/V1/Actors/BP_LoadBase.BP_LoadBase_C" :!class /Script/Engine.PrimitiveComponent)
      (bind _asbp_load_base (Utilities|Casting|CastToBP_LoadBase _array_element)
        (:then
          (Default|LoadBox _asbp_load_base)
          (Utilities|Array|Add _tempboxloc (Variables|/Script/Engine.SceneComponent|GetRelativeLocation (Variables|Default|GetC1)))
          (Utilities|Array|Add _tempboxloc (Variables|/Script/Engine.SceneComponent|GetRelativeLocation (Variables|Default|GetC2)))
          (Utilities|Array|Add _tempboxloc (Variables|/Script/Engine.SceneComponent|GetRelativeLocation (Variables|Default|GetC3)))
          (Utilities|Array|Add _tempboxloc (Variables|/Script/Engine.SceneComponent|GetRelativeLocation (Variables|Default|GetC4)))
          (Transformation|SetWorldLocation (Variables|Default|GetC1) (Transformation|GetWorldLocation (Variables|/Game/V1/Actors/BP_LoadBase.BP_LoadBase_C|GetC1 _asbp_load_base)) false false)
          (Transformation|SetWorldLocation (Variables|Default|GetC2) (Transformation|GetWorldLocation (Variables|/Game/V1/Actors/BP_LoadBase.BP_LoadBase_C|GetC2 _asbp_load_base)) false false)
          (Transformation|SetWorldLocation (Variables|Default|GetC3) (Transformation|GetWorldLocation (Variables|/Game/V1/Actors/BP_LoadBase.BP_LoadBase_C|GetC3 _asbp_load_base)) false false)
          (Transformation|SetWorldLocation (Variables|Default|GetC4) (Transformation|GetWorldLocation (Variables|/Game/V1/Actors/BP_LoadBase.BP_LoadBase_C|GetC4 _asbp_load_base)) false false)
          (Rendering|SetVisibility _c1 true false)
          (Components|MoveComponentTo _c1 (Utilities|Array|Get(acopy) (Variables|Default|GetTempBoxLoc)) "0, 0, 0" false false 2.0 false)
          (Rendering|SetVisibility _c2 true false)
          (Components|MoveComponentTo _c2 (Utilities|Array|Get(acopy) (Variables|Default|GetTempBoxLoc) 1) "0, 0, 0" false false 2.0 false)
          (Rendering|SetVisibility _c3 true false)
          (Components|MoveComponentTo _c3 (Utilities|Array|Get(acopy) (Variables|Default|GetTempBoxLoc) 2) "0, 0, 0" false false 2.0 false)
          (Rendering|SetVisibility _c4 true false)
          (Components|MoveComponentTo _c4 (Utilities|Array|Get(acopy) (Variables|Default|GetTempBoxLoc) 3) "0, 0, 0" false false 2.0 false))
        (:CastFailed
          (Development|PrintString "Cast Failed" true true "(R=1.000000,G=0.000000,B=0.000000,A=1.000000)"))))))

(event Input|KeyboardEvents|F
  (params (Key :type Key%20Structure :default "None"))
  ;[0 0 0] Comment
  ;;[0.1373 0.1373 0.1373] Upload containers
  (:Pressed
    (for _array_element (Collision|GetOverlappingActors (Variables|Default|GetCapsule) "/Game/V1/Actors/BP_UploadBase.BP_UploadBase_C" :!class /Script/Engine.PrimitiveComponent)
      (bind _asbp_upload_base (Utilities|Casting|CastToBP_UploadBase _array_element)
        (:then
          (Default|UploadBox _asbp_upload_base)
          (Rendering|Material|SetMaterial (Variables|Default|GetC1) 0 "/Engine/BasicShapes/BasicShapeMaterial.BasicShapeMaterial")
          (Utilities|FlowControl|Delay 1.5)
          (Rendering|Material|SetMaterial (Variables|Default|GetC2) 0 "/Engine/BasicShapes/BasicShapeMaterial.BasicShapeMaterial")
          (Utilities|FlowControl|Delay 1.5)
          (Rendering|Material|SetMaterial (Variables|Default|GetC3) 0 "/Engine/BasicShapes/BasicShapeMaterial.BasicShapeMaterial")
          (Utilities|FlowControl|Delay 1.5)
          (Rendering|Material|SetMaterial (Variables|Default|GetC4) 0 "/Engine/BasicShapes/BasicShapeMaterial.BasicShapeMaterial"))
        (:CastFailed
          (Development|PrintString "Cast Failed" true true "(R=1.000000,G=0.000000,B=0.000000,A=1.000000)"))))))

(fn ConstructionScript)

(fn UpdateText
  (Rendering|Components|TextRender|SetText (Variables|Default|GetTextCurrentAngle) (Utilities|Text|ToText(Float) (Variables|Default|GetCurrentAngle) "HalfToEven" false true 1 324 0 2))
  (Rendering|Components|TextRender|SetText (Variables|Default|GetTextCurrentSpeed) (Utilities|Text|ToText(Float) (Variables|Default|GetCurrentSpeed) "HalfToEven"))
  (Rendering|Components|TextRender|SetText (Variables|Default|GetTextSpeed) (Utilities|Text|ToText(Float) (Variables|Default|GetSpeed) "HalfToEven"))
  (Rendering|Components|TextRender|SetText (Variables|Default|GetTextAngle) (Utilities|Text|ToText(Float) (Variables|Default|GetAngle) "HalfToEven")))