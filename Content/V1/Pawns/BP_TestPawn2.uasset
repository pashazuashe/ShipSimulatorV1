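; BP_TestPawn2 is a test pawn that moves along its forward vector from player input.
; The MoveForward axis, scaled by a SpeedMultiplier variable, feeds a forced AddMovementInput call.
; MoveRight and Tick are empty, and unconnected AddMovementInput and SetActorLocation nodes remain in the graph without running.
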(event EventTick
  (params (DeltaSeconds :type Float%20%28single-precision%29)))

(event Input|AxisEvents|InputAxisMoveForward
  (params (AxisValue :type Float%20%28single-precision%29))
  (Pawn|Input|AddMovementInput (Transformation|GetActorForwardVector) (* AxisValue (Variables|Default|GetSpeedMultiplier)) true))

(event Input|AxisEvents|InputAxisMoveRight
  (params (AxisValue :type Float%20%28single-precision%29)))

(fn ConstructionScript)