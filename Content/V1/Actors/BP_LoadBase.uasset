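; BP_LoadBase is an actor that simulates loading boxes by hiding four components, C1 to C4, one after another.
; The custom LoadBox event hides each component in turn, using fixed delays to space out the steps.
; After the last delay it prints a message that the boxes are loaded; BeginPlay and the construction script are empty.
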(event Custom|LoadBox
  (Development|SetHiddeninGame (Variables|Default|GetC1) true false)
  (Utilities|FlowControl|Delay 2.0)
  (Development|SetHiddeninGame (Variables|Default|GetC2) true false)
  (Utilities|FlowControl|Delay 2.0)
  (Development|SetHiddeninGame (Variables|Default|GetC3) true false)
  (Utilities|FlowControl|Delay 2.0)
  (Development|SetHiddeninGame (Variables|Default|GetC4) true false)
  (Utilities|FlowControl|Delay 2.0)
  (Development|PrintString "box are loaded"))

(event EventBeginPlay)

(fn ConstructionScript)