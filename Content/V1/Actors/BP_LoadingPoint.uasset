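; BP_LoadingPoint is an actor with a point light and a box, apparently an unfinished overlap-trigger prototype.
; BeginPlay turns the light off; the begin-overlap handler prints debug text and lights it if OverlappedActor, rather than OtherActor, equals BP_DebugPawn.
; The overlap bindings, box overlap query and light-off branch are disconnected, so the graph never binds its handlers.
; End-overlap and Tick are empty, and no loading logic exists.
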(event Custom|OnActorBeginOverlap_Event
  (params (OverlappedActor :type Actor%20Object%20Reference) (OtherActor :type Actor%20Object%20Reference))
  (Development|PrintString "Hello")
  (if (== OverlappedActor "/Game/V1/Pawns/BP_DebugPawn.BP_DebugPawn")
    (Rendering|Components|Light|SetIntensity (Variables|Default|GetPointLight) 1e+03)
    (Development|PrintString "begin overlap")))

(event Custom|OnActorEndOverlap_Event
  (params (OverlappedActor :type Actor%20Object%20Reference) (OtherActor :type Actor%20Object%20Reference)))

(event EventBeginPlay
  (Rendering|Components|Light|SetIntensity (Variables|Default|GetPointLight) 0.0))

(event EventTick
  (params (DeltaSeconds :type Float%20%28single-precision%29)))

(fn ConstructionScript)