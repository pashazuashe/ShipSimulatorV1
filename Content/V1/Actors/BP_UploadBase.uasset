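; BP_UploadBase is an actor that shows a staged box upload by recoloring four components, C1 to C4.
; BeginPlay resets all four components to a basic shape material.
; The UploadBox event gives each component a different material in sequence with timed delays between steps, then prints a confirmation that the boxes are uploaded.
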(event Custom|UploadBox
  (Rendering|Material|SetMaterial (Variables|Default|GetC1) 0 "/Engine/MapTemplates/Materials/BasicAsset01.BasicAsset01")
  (Utilities|FlowControl|Delay 1.5)
  (Rendering|Material|SetMaterial (Variables|Default|GetC2) 0 "/Engine/MapTemplates/Materials/BasicAsset03.BasicAsset03")
  (Utilities|FlowControl|Delay 1.5)
  (Rendering|Material|SetMaterial (Variables|Default|GetC3) 0 "/Engine/MapTemplates/Materials/BasicAsset02.BasicAsset02")
  (Utilities|FlowControl|Delay 1.5)
  (Rendering|Material|SetMaterial (Variables|Default|GetC4) 0 "/DatasmithContent/Materials/CE_OpaqueReference.CE_OpaqueReference")
  (Development|PrintString "box are uploaded"))

(event EventBeginPlay
  (Rendering|Material|SetMaterial (Variables|Default|GetC1) 0 "/Engine/BasicShapes/BasicShapeMaterial.BasicShapeMaterial")
  (Rendering|Material|SetMaterial (Variables|Default|GetC2) 0 "/Engine/BasicShapes/BasicShapeMaterial.BasicShapeMaterial")
  (Rendering|Material|SetMaterial (Variables|Default|GetC3) 0 "/Engine/BasicShapes/BasicShapeMaterial.BasicShapeMaterial")
  (Rendering|Material|SetMaterial (Variables|Default|GetC4) 0 "/Engine/BasicShapes/BasicShapeMaterial.BasicShapeMaterial"))

(fn ConstructionScript)